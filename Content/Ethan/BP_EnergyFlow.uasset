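; Flow volume that carries characters and BP_PushableMove blocks along its forward vector, sized by LengthOfFlow in the construction script.
; Entering Collision zeroes a character's air control and gravity or stops a pushable's tick, then timelines lerp one horizontal coordinate to the flow's.
; Tick relaunches characters and sets pushable velocity until they leave the wider CollisionEnd, which restores character gravity.
; A box at the far end grants slight air control while overlapped.
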(event OnComponentBeginOverlap(Collision)
  (params (OverlappedComponent :type Primitive%20Component%20Object%20Reference) (OtherActor :type Actor%20Object%20Reference) (OtherComp :type Primitive%20Component%20Object%20Reference) (OtherBodyIndex :type Integer) (bFromSweep :type Boolean) (SweepResult :type Hit%20Result%20Structure%20%28by%20ref%29))
  (bind _returnvalue (Transformation|GetActorLocation))
  (bind _returnvalue_2 (Transformation|GetActorForwardVector))
  (bind _returnvalue_3 (Transformation|GetActorLocation OtherActor))
  (bind _returnvalue_4 (Transformation|GetActorForwardVector))
  (bind _returnvalue_5 (Transformation|GetActorLocation))
  (bind _returnvalue_6 (!= (.x _returnvalue_2) 0.0))
  (bind _returnvalue_7 (!= (.x _returnvalue_4) 0.0))
  (Utilities|Casting|CastToSphereComponent OtherComp
    (:CastFailed
      (bind _ascharacter (Utilities|Casting|CastToCharacter OtherActor)
        (:then
          (Utilities|Array|Add (Variables|Default|GetAffectedActors) OtherActor)
          (Variables|/Script/Engine.CharacterMovementComponent|SetAirControl (Variables|/Script/Engine.Character|GetCharacterMovement _ascharacter) 0.0)
          (Character|LaunchCharacter _ascharacter "0.000000,0.000000,50.000000" false true)
          (Utilities|FlowControl|Delay 0.05)
          (Variables|/Script/Engine.CharacterMovementComponent|SetGravityScale (Variables|/Script/Engine.Character|GetCharacterMovement _ascharacter) 0.0)
          (Components|Movement|StopMovementImmediately (Variables|/Script/Engine.Character|GetCharacterMovement _ascharacter))
          (Utilities|FlowControl|Delay 0.2)
          (bind _result (Timeline|ReCenter PlayFromStart)
            (:Update
              (Transformation|SetActorLocation _ascharacter (Math|Vector|Lerp(Vector) (Transformation|GetActorLocation _ascharacter) (Math|Vector|MakeVector (Math|Float|SelectFloat (.x _returnvalue_5) (.x (Transformation|GetActorLocation _ascharacter)) _returnvalue_7) (Math|Float|SelectFloat (.y (Transformation|GetActorLocation _ascharacter)) (.y _returnvalue_5) _returnvalue_7) (.z (Transformation|GetActorLocation _ascharacter))) _result) false false))))
        (:CastFailed
          (bind _asbp_pushable_move (Utilities|Casting|CastToBP_PushableMove OtherActor))
          (Utilities|Array|Add (Variables|Default|GetAffectedActors) OtherActor)
          (Utilities|FlowControl|Sequence
            (:then_0
              (Utilities|FlowControl|Delay 0.2)
              (Actor|Tick|SetActorTickEnabled _asbp_pushable_move))
            (:then_1
              (Utilities|FlowControl|Delay 0.2)
              (bind _result_2 (Timeline|Timeline PlayFromStart)
                (:Update
                  (Transformation|SetActorLocation OtherActor (Math|Vector|Lerp(Vector) (Transformation|GetActorLocation OtherActor) (Math|Vector|MakeVector (Math|Float|SelectFloat (.x _returnvalue) (.x _returnvalue_3) _returnvalue_6) (Math|Float|SelectFloat (.y _returnvalue_3) (.y _returnvalue) _returnvalue_6) (.z _returnvalue_3)) _result_2) false false))))))))))

(event OnComponentBeginOverlap(CollisionForAirControl)
  (params (OverlappedComponent :type Primitive%20Component%20Object%20Reference) (OtherActor :type Actor%20Object%20Reference) (OtherComp :type Primitive%20Component%20Object%20Reference) (OtherBodyIndex :type Integer) (bFromSweep :type Boolean) (SweepResult :type Hit%20Result%20Structure%20%28by%20ref%29))
  (Utilities|Casting|CastToSphereComponent OtherComp
    (:CastFailed
      (bind _ascharacter (Utilities|Casting|CastToCharacter OtherActor))
      (Variables|/Script/Engine.CharacterMovementComponent|SetAirControl (Variables|/Script/Engine.Character|GetCharacterMovement _ascharacter) 0.1))))

(event OnComponentEndOverlap(CollisionEnd)
  (params (OverlappedComponent :type Primitive%20Component%20Object%20Reference) (OtherActor :type Actor%20Object%20Reference) (OtherComp :type Primitive%20Component%20Object%20Reference) (OtherBodyIndex :type Integer))
  (Utilities|Casting|CastToSphereComponent OtherComp
    (:CastFailed
      (Utilities|Array|RemoveItem (Variables|Default|GetAffectedActors) OtherActor)
      (bind _ascharacter (Utilities|Casting|CastToCharacter OtherActor))
      (Variables|/Script/Engine.CharacterMovementComponent|SetGravityScale (Variables|/Script/Engine.Character|GetCharacterMovement _ascharacter) 1.75))))

(event OnComponentEndOverlap(CollisionForAirControl)
  (params (OverlappedComponent :type Primitive%20Component%20Object%20Reference) (OtherActor :type Actor%20Object%20Reference) (OtherComp :type Primitive%20Component%20Object%20Reference) (OtherBodyIndex :type Integer))
  (Utilities|Casting|CastToSphereComponent OtherComp
    (:CastFailed
      (bind _ascharacter (Utilities|Casting|CastToCharacter OtherActor))
      (Variables|/Script/Engine.CharacterMovementComponent|SetAirControl (Variables|/Script/Engine.Character|GetCharacterMovement _ascharacter) 0.0))))

(event EventBeginPlay
  (Components|Timeline|SetPlayRate (Variables|Default|GetReCenter) 2.0))

(event Collision|EventActorBeginOverlap
  (params (OtherActor :type Actor%20Object%20Reference)))

(event EventTick
  (params (DeltaSeconds :type Float%20%28single-precision%29))
  (for _array_element (Variables|Default|GetAffectedActors)
    (bind _ascharacter (Utilities|Casting|CastToCharacter _array_element)
      (:then
        (Character|LaunchCharacter _ascharacter (* (Transformation|GetActorForwardVector) (Variables|Default|GetPower)) false true))
      (:CastFailed
        (bind _asbp_pushable_move (Utilities|Casting|CastToBP_PushableMove _array_element))
        (Physics|SetPhysicsLinearVelocity (Variables|/Game/ThirdPerson/Blueprints/SceneObject/Pushable/BP_PushableMove.BP_PushableMove_C|GetCube _asbp_pushable_move) (* (Transformation|GetActorForwardVector) (Variables|Default|GetPowerBis)) false "None")))))

(fn ConstructionScript
  (Components|Box|SetBoxExtent (Variables|Default|GetCollision) (Math|Vector|MakeVector (Variables|Default|GetLengthOfFlow) 3e+01 3e+01) true)
  (Transformation|SetRelativeLocation (Variables|Default|GetCollision) (Math|Vector|MakeVector (Variables|Default|GetLengthOfFlow) 0.0 0.0) false false)
  (Components|Box|SetBoxExtent (Variables|Default|GetCollisionEnd) (Math|Vector|MakeVector (Variables|Default|GetLengthOfFlow) 1.5e+02 1.5e+02) true)
  (Transformation|SetRelativeLocation (Variables|Default|GetCollisionEnd) (Math|Vector|MakeVector (Variables|Default|GetLengthOfFlow) 0.0 0.0) false false)
  (Transformation|SetRelativeLocation (Variables|Default|GetCollisionForAirControl) (Math|Vector|MakeVector (* (Variables|Default|GetLengthOfFlow) 2.0) 0.0 0.0) false false)
  (Components|Box|SetBoxExtent (Variables|Default|GetCollisionForAirControl) (Math|Vector|MakeVector 5e+01 1.5e+02 1.5e+02) true))