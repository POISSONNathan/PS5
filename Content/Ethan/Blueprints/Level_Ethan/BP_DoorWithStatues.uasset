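; Puzzle door that opens once every statue in its AllTheStatues list is active.
; On BeginPlay it registers itself as each statue's Door and caches Door1's scale and Door2's location.
; CheckIfAllTheStatuesAreActive counts active statues; a full count sets IsOpen and plays a Timeline shrinking Door1 to zero scale while sliding Door2 to EndDoor2.
; Debug prints report the result, and nothing here closes the door again.
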(event Custom|CheckIfAllTheStatuesAreActive
  (bind _allthestatues (Variables|Default|GetAllTheStatues))
  (Variables|Default|SetActiveStatues 0)
  (for _array_element _allthestatues
    (if (Variables|/Game/Ethan/Blueprints/Level_Ethan/BP_AO_Statue.BP_AO_Statue_C|GetIsActive _array_element)
      (Math|Integer|IncrementInt (Variables|Default|GetActiveStatues))))
  (if (== (Variables|Default|GetActiveStatues) (Utilities|Array|Length _allthestatues))
    (Development|PrintString "Carrément je m'ouvre là")
    (Variables|Default|SetIsOpen true)
    (bind _newtrack_0 (Timeline|Timeline PlayFromStart)
      (:Update
        (Transformation|SetRelativeScale3D (Variables|Default|GetDoor1) (Math|Vector|Lerp(Vector) (Variables|Default|GetLocationDoor1) "0, 0, 0" _newtrack_0))
        (Transformation|SetRelativeLocation (Variables|Default|GetDoor2) (Math|Vector|Lerp(Vector) (Variables|Default|GetLocationDoor2) (Variables|/Script/Engine.SceneComponent|GetRelativeLocation (Variables|Default|GetEndDoor2)) _newtrack_0) false false)))
    (else
      (Development|PrintString "Azy jsuis fermé là"))))

(event EventBeginPlay
  (for _array_element (Variables|Default|GetAllTheStatues)
    (Variables|/Game/Ethan/Blueprints/Level_Ethan/BP_AO_Statue.BP_AO_Statue_C|SetDoor _array_element self)
    (Variables|Default|SetLocationDoor1 (Variables|/Script/Engine.SceneComponent|GetRelativeScale3D (Variables|Default|GetDoor1)))
    (Variables|Default|SetLocationDoor2 (Variables|/Script/Engine.SceneComponent|GetRelativeLocation (Variables|Default|GetDoor2)))))

(fn ConstructionScript)