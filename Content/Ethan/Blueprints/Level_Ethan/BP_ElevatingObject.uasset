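; Actionable level object that rises or moves to a preset spot when triggered, then returns after a fixed wait.
; The construction script gives Real and a PreVisualisation marker the same mesh; the marker is hidden at play and defines the destination.
; The overridden Action fires OnAction, where one timeline lerps Real to the marker and, after a delay, a second reverses it.
; CanPerform blocks retriggering until the return finishes.
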(event Custom|OnAction
  (if (Variables|Default|GetCanPerform?)
    (Variables|Default|SetCanPerform? false)
    (bind _newtrack_0 (Timeline|Elevate PlayFromStart)
      (:Update
        (Transformation|SetWorldLocation (Variables|Default|GetReal) (Math|Vector|Lerp(Vector) (Variables|Default|GetOriginalPosition) (Transformation|GetWorldLocation (Variables|Default|GetPreVisualisation)) _newtrack_0) false false))
      (:Finished
        (Utilities|FlowControl|Delay 15.0)
        (bind _newtrack_0_2 (Timeline|Delevate ReverseFromEnd)
          (:Update
            (Transformation|SetWorldLocation (Variables|Default|GetReal) (Math|Vector|Lerp(Vector) (Variables|Default|GetOriginalPosition) (Transformation|GetWorldLocation (Variables|Default|GetPreVisualisation)) _newtrack_0_2) false false))
          (:Finished
            (Variables|Default|SetCanPerform? true)))))))

(event EventBeginPlay
  (Variables|Default|SetOriginalPosition (Transformation|GetWorldLocation (Variables|Default|GetReal)))
  (Rendering|SetVisibility (Variables|Default|GetPreVisualisation) false false))

(event Collision|EventActorBeginOverlap
  (params (OtherActor :type Actor%20Object%20Reference)))

(event EventTick
  (params (DeltaSeconds :type Float%20%28single-precision%29)))

(fn ConstructionScript
  (Components|StaticMesh|SetStaticMesh (Variables|Default|GetReal) (Variables|Default|GetMesh))
  (Components|StaticMesh|SetStaticMesh (Variables|Default|GetPreVisualisation) (Variables|Default|GetMesh)))

(fn Action
  (|CallParentFunction)
  (CallFunction|OnAction))