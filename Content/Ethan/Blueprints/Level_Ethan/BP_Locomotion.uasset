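; Interactable spline-track ride that builds spline meshes along TheWay in the construction script.
; Interacting sends the player toward the Sit point via SimpleMoveToLocation, then waits a configurable delay.
; A FlipFlop alternates the Move timeline forward and in reverse, driving PointOnTheWay's position, pitch and yaw along the spline.
; Speed sets the timeline play rate, and finishing moves Sphere to the Locomotion component's location.
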(event EventBeginPlay
  (Components|Timeline|SetPlayRate (Variables|Default|GetMove) (Variables|Default|GetSpeed)))

(event Collision|EventActorBeginOverlap
  (params (OtherActor :type Actor%20Object%20Reference)))

(event EventTick
  (params (DeltaSeconds :type Float%20%28single-precision%29)))

(event EventInteractwith
  (bind _theway (Variables|Default|GetTheWay))
  (if (Variables|Default|GetCanGoBack)
    _
    (else
      (Utilities|FlowControl|DoOnce false
        (:Completed
          _))))
  (AI|Navigation|SimpleMovetoLocation (CallFunction|GetPlayerControlleras) (Transformation|GetWorldLocation (Variables|Default|GetSit)))
  (Utilities|FlowControl|Delay (Variables|Default|GetDelayBeforeStart))
  (Utilities|FlowControl|FlipFlop
    (:A
      (bind _newtrack_0 (Timeline|Move PlayFromStart)
        (:Update
          (Transformation|SetWorldLocation (Variables|Default|GetPointOnTheWay) (Spline|GetLocationatDistanceAlongSpline _theway (Math|Float|Lerp 0.0 (Spline|GetSplineLength _theway) _newtrack_0) "World") false false)
          (Transformation|SetWorldRotation (Variables|Default|GetPointOnTheWay) (Math|Rotator|MakeRotator 0.0 (.pitch (Spline|GetRotationatDistanceAlongSpline _theway (Math|Float|Lerp 0.0 (Spline|GetSplineLength _theway) _newtrack_0) "Local")) (.yaw (Spline|GetRotationatDistanceAlongSpline _theway (Math|Float|Lerp 0.0 (Spline|GetSplineLength _theway) _newtrack_0) "Local"))) false false))
        (:Finished
          (Transformation|SetWorldLocation (Variables|Default|GetSphere) (Transformation|GetWorldLocation (Variables|Default|GetLocomotion)) false false))))
    (:B
      (Timeline|Move ReverseFromEnd))))

(fn ConstructionScript
  (bind _theway (Variables|Default|GetTheWay))
  (for _index (range 0 (- (Spline|GetNumberOfSplinePoints (Variables|Default|GetTheWay)) 2))
    (bind _returnvalue (AddComponent|AddSplineMeshComponent false))
    (SplineMesh|SetStartandEnd _returnvalue (.Location (Spline|GetLocationandTangentatSplinePoint _theway _index "Local")) (.Tangent (Spline|GetLocationandTangentatSplinePoint _theway _index "Local")) (.Location (Spline|GetLocationandTangentatSplinePoint _theway (+ _index 1) "Local")) (.Tangent (Spline|GetLocationandTangentatSplinePoint _theway (+ _index 1) "Local")) true :!class /Script/Engine.SplineMeshComponent)
    (Transformation|AttachComponentToComponent _returnvalue (Variables|Default|GetDefaultSceneRoot) "None" "KeepRelative" "KeepRelative" "KeepRelative" true)))