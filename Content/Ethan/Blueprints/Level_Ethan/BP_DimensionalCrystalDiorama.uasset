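; Interactable crystal for the diorama level that switches the world between an original and a crystal dimension.
; Interacting plays a visual transition around a delayed physical switch, using timelines for a post-process radius via material parameter collection, custom depth and crystal glow.
; The physical switch flips the player's CrystalTurn and toggles visibility, gravity and collision profiles on each dimension's actors.
; With a linked crystal, it also shifts itself and the player by the offset between crystals, alternating direction.
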(event Custom|ActivateDimension
  (params (Dimension :type Actor%20Layer%20Structure) (IsActive :type Boolean) (NameOfTheDimension :type String))
  (bind _returnvalue (Class|LayersBlueprintLibrary|GetActors Dimension))
  (for _array_element _returnvalue
    (for _array_element_2 (Actor|GetComponentsByClass _array_element "/Script/Engine.PrimitiveComponent")
      (Rendering|SetVisibility _array_element_2 IsActive false)
      (Physics|SetEnableGravity _array_element_2 IsActive)
      (if IsActive
        (if (Utilities|Enum|Equal(Enum) NameOfTheDimension "OriginalDimension")
          (Collision|SetCollisionProfileName _array_element_2 "OriginalDimensionActive" true :!class /Script/Engine.PrimitiveComponent)
          (else
            (Collision|SetCollisionProfileName _array_element_2 "CrystalDimensionActive" true :!class /Script/Engine.PrimitiveComponent)))
        (elif (Utilities|Enum|Equal(Enum) NameOfTheDimension "CrystalDimension")
          (Collision|SetCollisionProfileName _array_element_2 "CrystalDimensionNotActive" true :!class /Script/Engine.PrimitiveComponent)
          (else
            (Collision|SetCollisionProfileName _array_element_2 "OriginalDimensionNotActive" true :!class /Script/Engine.PrimitiveComponent)))))))

(event Custom|DimensionVisualSwitch
  (Rendering|SetRenderCustomDepth (Variables|/Script/Engine.Character|GetMesh (.AsBP%20Third%20Person%20Diorama (Utilities|Casting|CastToBP_ThirdPersonDiorama (Game|Player|GetPlayerPawn 0)))) true)
  (Rendering|SetRenderCustomDepth (Variables|Default|GetStaticMesh5) true)
  (Rendering|SetRenderCustomDepth (Variables|Default|GetStaticMesh4) true)
  (Rendering|SetRenderCustomDepth (Variables|Default|GetStaticMesh3) true)
  (Rendering|SetRenderCustomDepth (Variables|Default|GetStaticMesh) true)
  (Rendering|SetRenderCustomDepth (Variables|Default|GetStaticMesh2) true)
  (Rendering|SetRenderCustomDepth (Variables|Default|GetSocle) true)
  (Rendering|SetRenderCustomDepth (Variables|Default|GetStaticMesh1) true)
  (Rendering|SetRenderCustomDepth (Variables|Default|GetMain) true)
  (Utilities|FlowControl|FlipFlop
    (:A
      (Rendering|Components|Light|SetLightColor (Variables|Default|GetPointLight) "(R=1.000000,G=1.000000,B=1.000000,A=1.000000)" true)
      (Rendering|Material|SetVectorParameterValue "/Game/Ethan/PostProcess/Collections/PC_PostProcess.PC_PostProcess" "Position" (Math|Conversions|ToLinearColor(Vector) (Transformation|GetActorLocation)) :!class /Script/Engine.KismetMaterialLibrary)
      (Utilities|FlowControl|Sequence
        (:then_0
          (Utilities|FlowControl|Delay 0.25)
          (bind _function (Timeline|Grow PlayFromStart)
            (:Update
              (Rendering|Material|SetScalarParameterValue "/Game/Ethan/PostProcess/Collections/PC_PostProcess.PC_PostProcess" "Radius" (Math|Float|Lerp 0.0 1e+04 _function) :!class /Script/Engine.KismetMaterialLibrary))
            (:Finished
              (bind _function_2 (Timeline|GrowBis PlayFromStart)
                (:Update
                  (Rendering|Material|SetScalarParameterValue "/Game/Ethan/PostProcess/Collections/PC_PostProcess.PC_PostProcess" "Radius" (Math|Float|Lerp 1e+04 5e+04 _function_2) :!class /Script/Engine.KismetMaterialLibrary))))))
        (:then_1
          (bind _function_3 (Timeline|Zoom PlayFromStart)))
        (:then_2
          (bind _function_4 (Timeline|Light PlayFromStart)
            (:Update
              (Rendering|Components|Light|SetIntensity (Variables|Default|GetPointLight) (Math|Float|Lerp 0.0 1e+06 _function_4))
              (Rendering|Material|SetScalarParameterValueonMaterials (Variables|Default|GetStaticMesh5) "EmissivePower" (/ (Math|Float|Lerp 0.0 1e+06 _function_4) 1e+03))
              (Rendering|Material|SetScalarParameterValueonMaterials (Variables|Default|GetStaticMesh4) "EmissivePower" (/ (Math|Float|Lerp 0.0 1e+06 _function_4) 1e+03))
              (Rendering|Material|SetScalarParameterValueonMaterials (Variables|Default|GetStaticMesh3) "EmissivePower" (/ (Math|Float|Lerp 0.0 1e+06 _function_4) 1e+03))
              (Rendering|Material|SetScalarParameterValueonMaterials (Variables|Default|GetStaticMesh) "EmissivePower" (/ (Math|Float|Lerp 0.0 1e+06 _function_4) 1e+03))
              (Rendering|Material|SetScalarParameterValueonMaterials (Variables|Default|GetStaticMesh2) "EmissivePower" (/ (Math|Float|Lerp 0.0 1e+06 _function_4) 1e+03))
              (Rendering|Material|SetScalarParameterValueonMaterials (Variables|Default|GetStaticMesh1) "EmissivePower" (/ (Math|Float|Lerp 0.0 1e+06 _function_4) 1e+03))
              (Rendering|Material|SetScalarParameterValueonMaterials (Variables|Default|GetMain) "EmissivePower" (/ (Math|Float|Lerp 0.0 1e+06 _function_4) 1e+03)))))))
    (:B
      (Rendering|Components|Light|SetLightColor (Variables|Default|GetPointLight) "(R=1.000000,G=1.000000,B=1.000000,A=1.000000)" true)
      (Rendering|Material|SetVectorParameterValue "/Game/Ethan/PostProcess/Collections/PC_PostProcess.PC_PostProcess" "Position" (Math|Conversions|ToLinearColor(Vector) (Transformation|GetActorLocation)) :!class /Script/Engine.KismetMaterialLibrary)
      (Utilities|FlowControl|Sequence
        (:then_0
          (Utilities|FlowControl|Delay 0.25)
          (bind _function_5 (Timeline|DeGrow PlayFromStart)
            (:Update
              (Rendering|Material|SetScalarParameterValue "/Game/Ethan/PostProcess/Collections/PC_PostProcess.PC_PostProcess" "Radius" (Math|Float|Lerp 1e+04 5e+04 _function_5) :!class /Script/Engine.KismetMaterialLibrary))
            (:Finished
              (bind _function_6 (Timeline|DeGrowBis ReverseFromEnd)
                (:Update
                  (Rendering|Material|SetScalarParameterValue "/Game/Ethan/PostProcess/Collections/PC_PostProcess.PC_PostProcess" "Radius" (Math|Float|Lerp 0.0 1e+04 _function_6) :!class /Script/Engine.KismetMaterialLibrary))
                (:Finished
                  (Rendering|SetRenderCustomDepth (Variables|Default|GetMain) false)
                  (Rendering|SetRenderCustomDepth (Variables|Default|GetStaticMesh5) false)
                  (Rendering|SetRenderCustomDepth (Variables|Default|GetStaticMesh4) false)
                  (Rendering|SetRenderCustomDepth (Variables|Default|GetStaticMesh3) false)
                  (Rendering|SetRenderCustomDepth (Variables|Default|GetStaticMesh) false)
                  (Rendering|SetRenderCustomDepth (Variables|Default|GetStaticMesh2) false)
                  (Rendering|SetRenderCustomDepth (Variables|Default|GetSocle) false)
                  (Rendering|SetRenderCustomDepth (Variables|Default|GetStaticMesh1) false))))))
        (:then_1
          (bind _function_7 (Timeline|DeZoom ReverseFromEnd)))
        (:then_2
          (bind _function_8 (Timeline|DeLight ReverseFromEnd)))))))

(event Custom|DimensionPhysicalSwitch
  (bind _returnvalue (Game|Player|GetPlayerPawn 0))
  (bind _asbp_third_person_character (CallFunction|GetPlayerCharacteras))
  (bind _asbp_third_person_character_2 (CallFunction|GetPlayerCharacteras))
  (bind _asbp_third_person_diorama (Utilities|Casting|CastToBP_ThirdPersonDiorama _returnvalue))
  (if (Variables|/Game/ThirdPerson/Blueprints/zDiorama/BP_ThirdPersonDiorama.BP_ThirdPersonDiorama_C|GetCrystalTurn _asbp_third_person_diorama)
    (Variables|/Game/ThirdPerson/Blueprints/zDiorama/BP_ThirdPersonDiorama.BP_ThirdPersonDiorama_C|SetCrystalTurn _asbp_third_person_diorama false)
    (CallFunction|ActivateDimension (Variables|Default|GetOriginalDimension) true)
    (CallFunction|ActivateDimension (Variables|Default|GetCrystalDimension) false)
    (else
      (Variables|/Game/ThirdPerson/Blueprints/zDiorama/BP_ThirdPersonDiorama.BP_ThirdPersonDiorama_C|SetCrystalTurn _asbp_third_person_diorama true)
      (CallFunction|ActivateDimension (Variables|Default|GetCrystalDimension) true)
      (CallFunction|ActivateDimension (Variables|Default|GetOriginalDimension) false)))
  (if (Utilities|IsValid (Variables|Default|GetLinkedCrystal))
    (Variables|/Script/Engine.SpringArmComponent|SetCameraLagSpeed (Variables|/Game/ThirdPerson/Blueprints/Player/BP_ThirdPersonCharacter.BP_ThirdPersonCharacter_C|GetCameraBoom (CallFunction|GetPlayerCharacteras)) 3.0)
    (if (Variables|Default|GetGoBack)
      (Transformation|SetActorLocation (- (Transformation|GetActorLocation) (Variables|Default|GetDistance)) false false)
      (Transformation|SetActorLocation _asbp_third_person_character (- (Transformation|GetActorLocation _asbp_third_person_character) (Variables|Default|GetDistance)) false false)
      (Variables|Default|SetGoBack false)
      (Variables|/Script/Engine.SpringArmComponent|SetCameraLagSpeed (Variables|/Game/ThirdPerson/Blueprints/Player/BP_ThirdPersonCharacter.BP_ThirdPersonCharacter_C|GetCameraBoom (CallFunction|GetPlayerCharacteras)) 2.0)
      (else
        (Transformation|SetActorLocation _asbp_third_person_character_2 (+ (Transformation|GetActorLocation _asbp_third_person_character_2) (Variables|Default|GetDistance)) false false)
        (Transformation|SetActorLocation (+ (Transformation|GetActorLocation) (Variables|Default|GetDistance)) false false)
        (Variables|Default|SetGoBack true)))))

(event Custom|SetUiFilter
  (if (Variables|/Game/ThirdPerson/Blueprints/Player/BP_ThirdPersonCharacter.BP_ThirdPersonCharacter_C|GetCrystalTurn (CallFunction|GetPlayerCharacteras))
    (bind _newtrack_0 (Timeline|Timeline PlayFromStart)
      (:Update
        (Default|UpdateFilterUi (Variables|/Game/ThirdPerson/Blueprints/zDiorama/BP_ThirdPersonDiorama.BP_ThirdPersonDiorama_C|GetUIDiorama (.AsBP%20Third%20Person%20Diorama (Utilities|Casting|CastToBP_ThirdPersonDiorama (Game|Player|GetPlayerPawn 0)))) _newtrack_0)))
    (else
      (Timeline|Timeline ReverseFromEnd))))

(event EventBeginPlay
  (bind _linkedcrystal (Variables|Default|GetLinkedCrystal))
  (Utilities|Array|Add (Variables|Default|GetDoNotDisapear) self)
  (Utilities|Array|Add (Variables|Default|GetDoNotDisapear) (Game|Player|GetPlayerPawn 0))
  (Components|Timeline|SetPlayRate (Variables|Default|GetGrow) 2.0)
  (Components|Timeline|SetPlayRate (Variables|Default|GetDeGrow) 1e+02)
  (Components|Timeline|SetPlayRate (Variables|Default|GetGrowBis) 1e+02)
  (Components|Timeline|SetPlayRate (Variables|Default|GetDeGrowBis) 1.5)
  (Components|Timeline|SetPlayRate (Variables|Default|GetZoom) 2.0)
  (Components|Timeline|SetPlayRate (Variables|Default|GetDeZoom) 2.0)
  (Components|Timeline|SetPlayRate (Variables|Default|GetLight) 2.0)
  (Components|Timeline|SetPlayRate (Variables|Default|GetDeLight) 2.0)
  (Utilities|FlowControl|Delay 0.1)
  (if (Utilities|IsValid (Variables|Default|GetLinkedCrystal))
    (Variables|Default|SetDistance (* (Math|Vector|GetUnitDirection(Vector) (Transformation|GetActorLocation) (Transformation|GetActorLocation _linkedcrystal)) (Transformation|GetDistanceTo _linkedcrystal self)))
    (Development|PrintString (Utilities|GetDisplayName (Variables|Default|GetLinkedCrystal)))))

(event Collision|EventActorBeginOverlap
  (params (OtherActor :type Actor%20Object%20Reference)))

(event EventTick
  (params (DeltaSeconds :type Float%20%28single-precision%29)))

(event EventInteractwith
  (if (Variables|Default|GetCanChange?)
    (Variables|Default|SetCanChange? false)
    (bind _isa (Utilities|FlowControl|FlipFlop)
      (:A
        _)
      (:B
        _))
    (Variables|Default|SetNewTurn? _isa)
    (CallFunction|DimensionVisualSwitch)
    (if (Utilities|IsValid (Variables|Default|GetLinkedCrystal))
      (Utilities|FlowControl|Delay 0.75)
      (else
        (Utilities|FlowControl|Delay 0.4)))
    (CallFunction|DimensionPhysicalSwitch)
    (if (Utilities|IsValid (Variables|Default|GetLinkedCrystal))
      (Utilities|FlowControl|Delay 0.5)
      (else
        (Utilities|FlowControl|Delay 0.2)))
    (CallFunction|DimensionVisualSwitch)
    (Utilities|FlowControl|Delay 1.0)
    (Variables|Default|SetCanChange? true)))

(fn ConstructionScript)