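; Rotating statue puzzle piece that reports to a Door once turned.
; Action triggers IfTouchByRed, which uses a timeline to lerp Sphere 90 degrees in yaw, ignoring input until finished.
; It then sets IsActive by a zero-tolerance match against GoodRotation, prints debug feedback and has Door recheck all statues.
; The construction script applies the start and target rotations to Sphere and Sphere1, the latter hidden at BeginPlay.
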(event Custom|IfTouchByRed
  (if (Variables|Default|GetCanRotate)
    (Variables|Default|SetCanRotate false)
    (bind _output_get (Variables|Default|SetActualRotation (Variables|/Script/Engine.SceneComponent|GetRelativeRotation (Variables|Default|GetSphere))))
    (Variables|Default|SetNewRotation (Math|Rotator|MakeRotator (.roll _output_get) (.pitch _output_get) (+ (.yaw _output_get) 9e+01)))
    (bind _function (Timeline|Rotate PlayFromStart)
      (:Update
        (Transformation|SetRelativeRotation (Variables|Default|GetSphere) (Math|Rotator|Lerp(Rotator) (Math|Rotator|MakeRotator (.roll (Variables|Default|GetActualRotation)) (.pitch (Variables|Default|GetActualRotation)) (.yaw (Variables|Default|GetActualRotation))) (Math|Rotator|MakeRotator (.roll (Variables|Default|GetNewRotation)) (.pitch (Variables|Default|GetNewRotation)) (.yaw (Variables|Default|GetNewRotation))) _function) false false))
      (:Finished
        (Variables|Default|SetCanRotate true)
        (Variables|Default|SetActualRotation (Variables|/Script/Engine.SceneComponent|GetRelativeRotation (Variables|Default|GetSphere)))
        (if (Utilities|Operators|EqualEqual (Variables|Default|GetActualRotation) (Variables|Default|GetGoodRotation) 0.0)
          (Variables|Default|SetIsActive true)
          (Development|PrintString "C'est bon wesh")
          (else
            (Variables|Default|SetIsActive false)
            (Development|PrintString "Essaie encore mon reuf")))
        (Default|CheckifAlltheStatuesAreActive (Variables|Default|GetDoor))))))

(event EventBeginPlay
  (Rendering|SetVisibility (Variables|Default|GetSphere1) false true))

(event Collision|EventActorBeginOverlap
  (params (OtherActor :type Actor%20Object%20Reference)))

(event EventTick
  (params (DeltaSeconds :type Float%20%28single-precision%29)))

(fn ConstructionScript
  (Transformation|SetRelativeRotation (Variables|Default|GetSphere1) (Variables|Default|GetGoodRotation) false false)
  (Transformation|SetRelativeRotation (Variables|Default|GetSphere) (Variables|Default|GetActualRotation) false false))

(fn Action
  (|CallParentFunction)
  (CallFunction|IfTouchbyRed))