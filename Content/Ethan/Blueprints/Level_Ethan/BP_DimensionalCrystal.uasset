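; Interactable crystal that toggles the level between an original dimension and a crystal dimension, tracked by the player's CrystalTurn flag.
; On interact, it hides every actor outside the DoNotDisapear list (which gains itself and the player at BeginPlay), swaps dimensions after a short delay, then unhides them.
; ActivateDimension switches each primitive component's visibility, gravity and collision response (Block or Overlap on all channels) for that dimension's actors.
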(event Custom|ActivateDimension
  (params (Dimension :type Actor%20Layer%20Structure) (IsActive :type Boolean))
  (bind _returnvalue (Class|LayersBlueprintLibrary|GetActors Dimension))
  (for _array_element _returnvalue
    (for _array_element_2 (Actor|GetComponentsByClass _array_element "/Script/Engine.PrimitiveComponent")
      (if IsActive
        (Collision|SetCollisionResponsetoAllChannels _array_element_2 "ECR_Block")
        (else
          (Collision|SetCollisionResponsetoAllChannels _array_element_2 "ECR_Overlap")))
      (Development|SetHiddeninGame _array_element_2 (not IsActive) false)
      (Physics|SetEnableGravity _array_element_2 IsActive))))

(event EventBeginPlay
  (Utilities|Array|Add (Variables|Default|GetDoNotDisapear) self)
  (Utilities|Array|Add (Variables|Default|GetDoNotDisapear) (CallFunction|GetPlayerCharacteras)))

(event Collision|EventActorBeginOverlap
  (params (OtherActor :type Actor%20Object%20Reference)))

(event EventTick
  (params (DeltaSeconds :type Float%20%28single-precision%29)))

(event EventInteractwith
  (bind _asbp_third_person_character (CallFunction|GetPlayerCharacteras))
  (bind _outactors (Actor|GetAllActorsOfClass "/Script/Engine.Actor"))
  (for _array_element _outactors
    (if (not (Utilities|Array|ContainsItem (Variables|Default|GetDoNotDisapear) _array_element))
      (Rendering|SetActorHiddenInGame _array_element true)))
  (Utilities|FlowControl|Delay 0.5)
  (if (Variables|/Game/ThirdPerson/Blueprints/Player/BP_ThirdPersonCharacter.BP_ThirdPersonCharacter_C|GetCrystalTurn _asbp_third_person_character)
    (Variables|/Game/ThirdPerson/Blueprints/Player/BP_ThirdPersonCharacter.BP_ThirdPersonCharacter_C|SetCrystalTurn _asbp_third_person_character false)
    (CallFunction|ActivateDimension (Variables|Default|GetOriginalDimension) true)
    (CallFunction|ActivateDimension (Variables|Default|GetCrystalDimension) false)
    (else
      (Variables|/Game/ThirdPerson/Blueprints/Player/BP_ThirdPersonCharacter.BP_ThirdPersonCharacter_C|SetCrystalTurn _asbp_third_person_character true)
      (CallFunction|ActivateDimension (Variables|Default|GetCrystalDimension) true)
      (CallFunction|ActivateDimension (Variables|Default|GetOriginalDimension) false)))
  (bind _outactors_2 (Actor|GetAllActorsOfClass "/Script/Engine.Actor"))
  (for _array_element_2 _outactors_2
    (if (not (Utilities|Array|ContainsItem (Variables|Default|GetDoNotDisapear) _array_element_2))
      (Rendering|SetActorHiddenInGame _array_element_2 false))))

(fn ConstructionScript)