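; Directional energy stream that carries characters, pushable blocks and crystals along its forward vector.
; Entering the inner box suspends character gravity or pushable tick, registers the actor and runs a recentering timeline through DirectionReCenter.
; Tick drives registered actors by launch or physics velocity until they leave the wider box, which restores character gravity.
; LengthOfFlow sizes the boxes in construction, placing an air-control zone at the far end.
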(event OnComponentBeginOverlap(Collision)
  (params (OverlappedComponent :type Primitive%20Component%20Object%20Reference) (OtherActor :type Actor%20Object%20Reference) (OtherComp :type Primitive%20Component%20Object%20Reference) (OtherBodyIndex :type Integer) (bFromSweep :type Boolean) (SweepResult :type Hit%20Result%20Structure%20%28by%20ref%29))
  (Utilities|Casting|CastToSphereComponent OtherComp
    (:then
      (bind _asbp_original_crystal (Utilities|Casting|CastToBP_OriginalCrystal OtherActor))
      (Utilities|FlowControl|Sequence
        (:then_0
          (Utilities|FlowControl|Delay 0.1)
          (Physics|SetPhysicsLinearVelocity (Variables|/Game/ThirdPerson/Blueprints/CrystalEffect/BP_OriginalCrystal.BP_OriginalCrystal_C|GetSphere _asbp_original_crystal) "0, 0, 0" false "None")
          (Utilities|Array|Add (Variables|Default|GetAffectedActors) OtherActor))
        (:then_1
          (Utilities|FlowControl|Delay 0.1)
          (bind _result (Timeline|RecenterBisBis PlayFromStart)
            (:Update
              (if (Utilities|IsValid OtherActor)
                (Transformation|SetActorLocation OtherActor (Utilities|DirectionReCenter _result OtherActor) false false)))))))
    (:CastFailed
      (bind _ascharacter (Utilities|Casting|CastToCharacter OtherActor)
        (:then
          (Utilities|Array|Add (Variables|Default|GetAffectedActors) OtherActor)
          (Variables|/Script/Engine.CharacterMovementComponent|SetAirControl (Variables|/Script/Engine.Character|GetCharacterMovement _ascharacter) 0.0)
          (Character|LaunchCharacter _ascharacter "0.000000,0.000000,50.000000" false true)
          (Utilities|FlowControl|Delay 0.05)
          (Variables|/Script/Engine.CharacterMovementComponent|SetGravityScale (Variables|/Script/Engine.Character|GetCharacterMovement _ascharacter) 0.0)
          (Components|Movement|StopMovementImmediately (Variables|/Script/Engine.Character|GetCharacterMovement _ascharacter))
          (Utilities|FlowControl|Delay 0.2)
          (bind _result_2 (Timeline|ReCenter PlayFromStart)
            (:Update
              (Transformation|SetActorLocation _ascharacter (Utilities|DirectionReCenter _result_2 _ascharacter) false false))))
        (:CastFailed
          (bind _asbp_pushable_move (Utilities|Casting|CastToBP_PushableMove OtherActor))
          (Utilities|FlowControl|Sequence
            (:then_0
              (Utilities|FlowControl|Delay 0.2)
              (Actor|Tick|SetActorTickEnabled _asbp_pushable_move)
              (Utilities|Array|Add (Variables|Default|GetAffectedActors) OtherActor))
            (:then_1
              (Utilities|FlowControl|Delay 0.2)
              (bind _result_3 (Timeline|RecenterBis PlayFromStart)
                (:Update
                  (Transformation|SetActorLocation OtherActor (Utilities|DirectionReCenter _result_3 OtherActor) false false))))))))))

(event OnComponentBeginOverlap(CollisionForAirControl)
  (params (OverlappedComponent :type Primitive%20Component%20Object%20Reference) (OtherActor :type Actor%20Object%20Reference) (OtherComp :type Primitive%20Component%20Object%20Reference) (OtherBodyIndex :type Integer) (bFromSweep :type Boolean) (SweepResult :type Hit%20Result%20Structure%20%28by%20ref%29))
  (Utilities|Casting|CastToSphereComponent OtherComp
    (:CastFailed
      (bind _ascharacter (Utilities|Casting|CastToCharacter OtherActor))
      (Variables|/Script/Engine.CharacterMovementComponent|SetAirControl (Variables|/Script/Engine.Character|GetCharacterMovement _ascharacter) 0.1))))

(event OnComponentEndOverlap(CollisionEnd)
  (params (OverlappedComponent :type Primitive%20Component%20Object%20Reference) (OtherActor :type Actor%20Object%20Reference) (OtherComp :type Primitive%20Component%20Object%20Reference) (OtherBodyIndex :type Integer))
  (Utilities|Casting|CastToSphereComponent OtherComp
    (:then
      (Utilities|Casting|CastToBP_OriginalCrystal OtherActor)
      (Utilities|Array|RemoveItem (Variables|Default|GetAffectedActors) OtherActor))
    (:CastFailed
      (Utilities|Array|RemoveItem (Variables|Default|GetAffectedActors) OtherActor)
      (bind _ascharacter (Utilities|Casting|CastToCharacter OtherActor))
      (Variables|/Script/Engine.CharacterMovementComponent|SetGravityScale (Variables|/Script/Engine.Character|GetCharacterMovement _ascharacter) 1.75))))

(event OnComponentEndOverlap(CollisionForAirControl)
  (params (OverlappedComponent :type Primitive%20Component%20Object%20Reference) (OtherActor :type Actor%20Object%20Reference) (OtherComp :type Primitive%20Component%20Object%20Reference) (OtherBodyIndex :type Integer))
  (Utilities|Casting|CastToSphereComponent OtherComp
    (:CastFailed
      (bind _ascharacter (Utilities|Casting|CastToCharacter OtherActor))
      (Variables|/Script/Engine.CharacterMovementComponent|SetAirControl (Variables|/Script/Engine.Character|GetCharacterMovement _ascharacter) 0.0))))

(event EventBeginPlay
  (Components|Timeline|SetPlayRate (Variables|Default|GetReCenter) 2.0)
  (Components|Timeline|SetPlayRate (Variables|Default|GetRecenterBis) 2.0)
  (Components|Timeline|SetPlayRate (Variables|Default|GetReCenter) 2.0))

(event Collision|EventActorBeginOverlap
  (params (OtherActor :type Actor%20Object%20Reference)))

(event EventTick
  (params (DeltaSeconds :type Float%20%28single-precision%29))
  (for _array_element (Variables|Default|GetAffectedActors)
    (bind _ascharacter (Utilities|Casting|CastToCharacter _array_element)
      (:then
        (Character|LaunchCharacter _ascharacter (* (Transformation|GetActorForwardVector) (Variables|Default|GetPower)) false true))
      (:CastFailed
        (bind _asbp_pushable_move (Utilities|Casting|CastToBP_PushableMove _array_element)
          (:then
            (Physics|SetPhysicsLinearVelocity (Variables|/Game/ThirdPerson/Blueprints/SceneObject/Pushable/BP_PushableMove.BP_PushableMove_C|GetCube _asbp_pushable_move) (* (Transformation|GetActorForwardVector) (Variables|Default|GetPowerBis)) false "None"))
          (:CastFailed
            (bind _asbp_original_crystal (Utilities|Casting|CastToBP_OriginalCrystal _array_element))
            (Physics|SetPhysicsLinearVelocity (Variables|/Game/ThirdPerson/Blueprints/CrystalEffect/BP_OriginalCrystal.BP_OriginalCrystal_C|GetSphere _asbp_original_crystal) (* (Transformation|GetActorForwardVector) (Variables|Default|GetPowerBis)) false "None")))))))

(fn ConstructionScript
  (Components|Box|SetBoxExtent (Variables|Default|GetCollision) (Math|Vector|MakeVector (Variables|Default|GetLengthOfFlow) 3e+01 3e+01) true)
  (Transformation|SetRelativeLocation (Variables|Default|GetCollision) (Math|Vector|MakeVector (Variables|Default|GetLengthOfFlow) 0.0 0.0) false false)
  (Components|Box|SetBoxExtent (Variables|Default|GetCollisionEnd) (Math|Vector|MakeVector (Variables|Default|GetLengthOfFlow) 1.5e+02 1.5e+02) true)
  (Transformation|SetRelativeLocation (Variables|Default|GetCollisionEnd) (Math|Vector|MakeVector (Variables|Default|GetLengthOfFlow) 0.0 0.0) false false)
  (Transformation|SetRelativeLocation (Variables|Default|GetCollisionForAirControl) (Math|Vector|MakeVector (* (Variables|Default|GetLengthOfFlow) 2.0) 0.0 0.0) false false)
  (Components|Box|SetBoxExtent (Variables|Default|GetCollisionForAirControl) (Math|Vector|MakeVector 5e+01 1.5e+02 1.5e+02) true))