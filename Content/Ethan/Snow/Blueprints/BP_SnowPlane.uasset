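; BP_SnowPlane is a snow surface actor that records left and right footprints into the RT_SnowPlane render target.
; On BeginPlay it creates a dynamic instance of the M_FootBrush_Inst brush material and clears the render target to black.
; Its Draw event takes 2D positions for each foot, writes them to the brush's Right and Left vector parameters, and draws the brush into the render target after each.
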(event Custom|Draw
  (params (Right :type Vector%202D%20Structure) (Left :type Vector%202D%20Structure))
  (bind _brushref (Variables|Default|GetBrushRef))
  (bind _brushref_2 (Variables|Default|GetBrushRef))
  (Utilities|FlowControl|Sequence
    (:then_0
      (Rendering|Material|SetVectorParameterValue _brushref_2 "Right" (Math|Conversions|ToLinearColor(Vector) (Math|Conversions|ToVector(Vector2D) Right)) :!class /Script/Engine.MaterialInstanceDynamic)
      (Rendering|DrawMaterialtoRenderTarget "/Game/Ethan/Snow/Textures/RT_SnowPlane.RT_SnowPlane" _brushref_2))
    (:then_1
      (Rendering|Material|SetVectorParameterValue _brushref "Left" (Math|Conversions|ToLinearColor(Vector) (Math|Conversions|ToVector(Vector2D) Left)) :!class /Script/Engine.MaterialInstanceDynamic)
      (Rendering|DrawMaterialtoRenderTarget "/Game/Ethan/Snow/Textures/RT_SnowPlane.RT_SnowPlane" _brushref))))

(event EventBeginPlay
  (bind _returnvalue (Rendering|Material|CreateDynamicMaterialInstance "/Game/Ethan/Snow/Materials/M_FootBrush_Inst.M_FootBrush_Inst" "None" "None" :!class /Script/Engine.KismetMaterialLibrary))
  (Variables|Default|SetBrushRef _returnvalue)
  (Rendering|ClearRenderTarget2D "/Game/Ethan/Snow/Textures/RT_SnowPlane.RT_SnowPlane"))

(event Collision|EventActorBeginOverlap
  (params (OtherActor :type Actor%20Object%20Reference)))

(event EventTick
  (params (DeltaSeconds :type Float%20%28single-precision%29)))

(fn ConstructionScript)