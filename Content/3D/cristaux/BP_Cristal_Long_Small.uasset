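; Long small crystal prop whose point light and emissive material glow fluctuate randomly from the start of play.
; A looping event picks random targets for light intensity and the Emissive parameter, then a timeline blends both from their current values.
; When the timeline finishes, it stores the targets as current, waits a short random delay and calls the event again.
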(event Custom|ChangeEmissiveAndLight*
  (bind _returnvalue (Math|Random|RandomFloatinRange 0.0 1e+02))
  (bind _returnvalue_2 (/ _returnvalue 1e+02))
  (Variables|Default|SetNewEmissive (Math|Float|Lerp 1.0 2.5 _returnvalue_2))
  (Variables|Default|SetNewIntensity (Math|Float|Lerp 1.5e+03 1e+04 _returnvalue_2))
  (bind _newtrack_0 (Timeline|Timeline PlayFromStart)
    (:Update
      (Rendering|Components|Light|SetIntensity (Variables|Default|GetPointLight) (Math|Float|Lerp (Variables|Default|GetCurrentIntensity) (Variables|Default|GetNewIntensity) _newtrack_0))
      (Rendering|Material|SetScalarParameterValueonMaterials (Variables|Default|GetSM_Long_Small_Crystal_Nod) "Emissive" (Math|Float|Lerp (Variables|Default|GetCurrentEmissive) (Variables|Default|GetNewEmissive) _newtrack_0)))
    (:Finished
      (Variables|Default|SetCurrentIntensity (Variables|Default|GetNewIntensity))
      (Variables|Default|SetCurrentEmissive (Variables|Default|GetNewEmissive))
      (Utilities|FlowControl|Delay (Math|Random|RandomFloatinRange 0.0 0.4))
      (CallFunction|ChangeEmissiveandLight*))))

(event EventBeginPlay
  (CallFunction|ChangeEmissiveandLight*))

(fn ConstructionScript)